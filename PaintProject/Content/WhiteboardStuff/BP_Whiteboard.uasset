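; Whiteboard actor that paints marker marks onto a render target where the mouse cursor points.
; BeginPlay creates a dynamic marker material and clears the render target.
; Each Tick traces from the cursor, converts any whiteboard hit to a collision UV, and draws the marker material there via its DrawLocation parameter.
; Right mouse toggles IsDrawing while held, but Tick draws without checking it.
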(event Custom|Draw%20on%20whiteboard
  (params (DrawLOC :type Vector%202D%20Structure))
  (bind _marker_mi (Variables|Default|GetMarker_MI))
  (Rendering|Material|SetVectorParameterValue _marker_mi "DrawLocation" (Math|Conversions|ToLinearColor(Vector) (Math|Conversions|ToVector(Vector2D) DrawLOC)) :!class /Script/Engine.MaterialInstanceDynamic)
  (Rendering|DrawMaterialtoRenderTarget "/Game/WhiteboardStuff/RT_whiteboard.RT_whiteboard" _marker_mi))

(event EventBeginPlay
  (bind _returnvalue (Rendering|Material|CreateDynamicMaterialInstance "/Game/WhiteboardStuff/M_Marker.M_Marker" "None" "None" :!class /Script/Engine.KismetMaterialLibrary))
  (Variables|Default|SetMarker_MI _returnvalue)
  (Rendering|ClearRenderTarget2D "/Game/WhiteboardStuff/RT_whiteboard.RT_whiteboard"))

(event EventTick
  (params (DeltaSeconds :type Float%20%28single-precision%29))
  (bind _returnvalue (Class|GameplayStatics|GetPlayerControllerfromID))
  (bind (_outhit _returnvalue_2) (Collision|LineTraceByChannel (.WorldLocation (Game|Player|ConvertMouseLocationToWorldSpace _returnvalue)) (* (.ImpactPoint (Collision|BreakHitResult (.HitResult (Game|Player|GetHitResultUnderCursorbyChannel _returnvalue "TraceTypeQuery1" true)))) 1.1) "TraceTypeQuery1" true 0 "ForDuration"))
  (if _returnvalue_2
    (bind _asbp_whiteboard (Utilities|Casting|CastToBP_Whiteboard (.HitActor (Collision|BreakHitResult _outhit)))
      (:then
        (CallFunction|DrawonWhiteboard _asbp_whiteboard (.UV (Class|GameplayStatics|FindCollisionUV _outhit))))
      (:CastFailed
        (Development|PrintString "Whiteboard Cast Failed")))))

(event Input|MouseEvents|RightMouseButton
  (params (Key :type Key%20Structure :default "None"))
  (:Pressed
    (Variables|Default|SetIs%20Drawing true))
  (:Released
    (Variables|Default|SetIs%20Drawing false)))

(fn ConstructionScript)